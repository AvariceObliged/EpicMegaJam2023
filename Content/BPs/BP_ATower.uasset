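; BP_ATower is a tower actor that fires at the first-person character when it enters the TowerRange component.
; On that overlap it prints a debug message, turns Base in yaw only toward the character and spawns one BP_ATowerBullet at the Turret's location.
; The spawn transform takes only that location, not the aim rotation.
; There is no tracking or repeat fire, so each new overlap yields a single shot.
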(event `self.TowerRange.OnComponentBeginOverlap`
  (params (OverlappedComponent :type "PrimitiveComponent Object Reference") (OtherActor :type "Actor Object Reference") (OtherComp :type "PrimitiveComponent Object Reference") (OtherBodyIndex :type Integer) (bFromSweep :type Boolean) (SweepResult :type "HitResult Structure (by ref)"))
  (bind (_returnvalue_roll _returnvalue_pitch _returnvalue_yaw) (`KismetMathLibrary.BreakRotator` (`KismetMathLibrary.FindLookAtRotation` (`self.K2_GetActorLocation`) (`self.K2_GetActorLocation` OtherActor))))
  (if (`GameplayStatics.ObjectIsA` OtherActor "/Game/FirstPerson/Blueprints/BP_FirstPersonCharacter.BP_FirstPersonCharacter_C")
    (`KismetSystemLibrary.PrintString` "I'm shooting a enemy")
    (`SceneComponent.K2_SetRelativeRotation` (`self.Base`) (`KismetMathLibrary.MakeRotator` 0.0 0.0 _returnvalue_yaw) false false)
    (`|SpawnActorFromClass` "/Game/BPs/BP_ATowerBullet.BP_ATowerBullet_C" (`KismetMathLibrary.Conv_VectorToTransform` (`SceneComponent.K2_GetComponentLocation` (`self.Turret`))) "Undefined" "MultiplyWithRoot" null null)))

(fn `UserConstructionScript`)