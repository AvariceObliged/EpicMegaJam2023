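; BP_BaseActor is an actor with health that takes damage when a class-checked actor overlaps its MeleeSphere.
; A hit subtracts TempDamage from Health, plays warning and alarm sounds, prints the remaining health and destroys the overlapping actor.
; An any-damage handler joins the same logic, ignoring its Damage input, but its only visible binding node sits inside the handler itself.
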(event `self.MeleeSphere.OnComponentBeginOverlap`
  (params (OverlappedComponent :type "PrimitiveComponent Object Reference") (OtherActor :type "Actor Object Reference") (OtherComp :type "PrimitiveComponent Object Reference") (OtherBodyIndex :type Integer) (bFromSweep :type Boolean) (SweepResult :type "HitResult Structure (by ref)"))
  (bind _health (`self.Health`))
  (bind _tempdamage (`self.tempDamage`))
  (if (`GameplayStatics.ObjectIsA` OtherActor)
    (set `self.Health` (- _health _tempdamage) :!label _label)
    (`GameplayStatics.PlaySound2D` "/Game/JamContent/Art/Audio/SFX/warning.warning" 1.0 1.0 0.0 null null)
    (`KismetSystemLibrary.PrintText` (`|FormatText` "I have taken {damage} damage. I have {hp} left" _tempdamage _health))
    (`GameplayStatics.PlaySoundAtLocation` "/Game/Audio/SFX/sci-fi-alarm-facility-02.sci-fi-alarm-facility-02" (0.0 0.0 0.0) (struct) 1.0 1.0 0.0 null null null null)
    (`self.K2_DestroyActor` OtherActor)))

(event `OnTakeAnyDamage_Event` :!signature `self.OnTakeAnyDamage`
  (params (DamagedActor :type "Actor Object Reference") (Damage :type "Float (single-precision)") (DamageType :type "DamageType Object Reference") (InstigatedBy :type "Controller Object Reference") (DamageCauser :type "Actor Object Reference"))
  (`KismetSystemLibrary.PrintString` "actor called")
  (add `self.OnTakeAnyDamage` (delegate `OnTakeAnyDamage_Event`))
  (goto _label))

(fn `UserConstructionScript`)