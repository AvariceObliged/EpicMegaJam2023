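; BP_WavePathingComponent walks its owning pawn along a waypoint path, then destroys it and damages the base.
; BeginPathing issues AI MoveTo requests one waypoint at a time, advancing on each successful completion and using CanFly to select the navigation filter.
; At path end, or when a move fails, it destroys the pawn, subtracts Health from BP_BaseActor and plays an alarm sound.
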(event `Begin Pathing`
  (params (Path :type "/Game/JamContent/BPs/Actors/BP_WavePathActor Object Reference"))
  (set `self.Path` Path)
  (bind _aspawn (cast `Pawn` (`self.GetOwner`))
    (:`then`
      (bind _output_get (set `self.Pawn` _aspawn))
      (add `AIController.ReceiveMoveCompleted` (`AIBlueprintHelperLibrary.GetAIController` _output_get) (delegate `CustomEvent`))
      (if (< (`self.NextWaypointIndex`) (`/Game/JamContent/BPs/Actors/BP_WavePathActor.GetWaypointCount` (`self.Path`))) :!label _label
        (`AIController.MoveToLocation` (`AIBlueprintHelperLibrary.GetAIController` (`self.Pawn`)) (`/Game/JamContent/BPs/Actors/BP_WavePathActor.GetWaypointLocation` (`self.Path`) (`self.NextWaypointIndex`)) 5.0 true true false true (select `bool` (`self.CanFly`) :`false` "/Game/JamContent/BPs/Navigation/NavQuery_Flightless.NavQuery_Flightless_C" :`true` "/Script/AIModule.NavFilter_AIControllerDefault" :!type "NavigationQueryFilter Class Reference") true)
        (else
          (`Actor.K2_DestroyActor` (`self.Pawn`) :!label _label_2)
          (`self.GetBaseActorAndDamage`))))
    (:`CastFailed`
      (`KismetSystemLibrary.PrintText` "BP_WavePathing not attached to Pawn actor" true true (struct :`R` 0.8 :`A` 1.0))
      (goto _label_2))))

(event `CustomEvent`
  (params (RequestID :type "AIRequestID Structure") (Result :type "EPathFollowingResult Enum" :default "Success"))
  (if (== Result 0)
    (set `self.NextWaypointIndex` (+ (`self.NextWaypointIndex`) 1))
    (goto _label)
    (else
      (`KismetSystemLibrary.PrintText` (`|FormatText` "AI MoveTo Failed: {Result}" (`|GetEnumeratorNameAsString` Result)) true true (struct :`R` 0.9 :`A` 1.0))
      (goto _label_2))))

(fn `GetBaseActorAndDamage`
  (bind _returnvalue (`GameplayStatics.GetActorOfClass` "/Game/BPs/BP_BaseActor.BP_BaseActor_C"))
  (set `/Game/BPs/BP_BaseActor.Health` (- (`/Game/BPs/BP_BaseActor.Health` _returnvalue) 0.05) _returnvalue)
  (`GameplayStatics.PlaySoundAtLocation` "/Game/Audio/SFX/sci-fi-alarm-facility-02.sci-fi-alarm-facility-02" (0.0 0.0 0.0) (struct) 1.0 1.0 0.0 null null null null))