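; Weapon component for the Melt Rifle, a hold-to-charge laser gun that damages enemies along the player's aim.
; Holding the charge input accumulates stored tick delta time while the weapon is ready, reporting progress to the owner; cancelling resets it.
; When CanFire passes, a multi sphere trace along the camera forward damages enemy hits and sparks every hit.
; It then calls ReloadGun and draws a Niagara beam to the final impact point.
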(event `self.ReceiveTick`
  (params (DeltaSeconds :type "Float (single-precision)"))
  (set `self.deltaT` DeltaSeconds))

(event `EnhancedInput|/Game/FirstPerson/Input/Actions/IA_ChargeShoot`
  (params (ActionValue :type Boolean) (ElapsedSeconds :type "Float (double-precision)") (TriggeredSeconds :type "Float (double-precision)") (InputAction :type "InputAction Object Reference" :default "/Game/FirstPerson/Input/Actions/IA_ChargeShoot.IA_ChargeShoot"))
  (:`Triggered`
    (if ActionValue
      (`self.ChargeGun`)
      (else
        (`self.CancelCharge`)))))

(fn `CancelCharge`
  (bind _output_get (set `self.CurrentCharge` 0.0))
  (`/Game/FirstPerson/Blueprints/BP_FirstPersonCharacter.OnChargeChanged` (`self.Owner`) _output_get))

(fn `ChargeGun`
  (if (`self.WeaponReady`)
    (if (== (`self.CurrentCharge`) 0.0)
      (`GameplayStatics.PlaySoundAtLocation` (`self.ReloadSound`) (`Actor.K2_GetActorLocation` (`self.Owner`)) (struct) 1.0 1.0 0.0 null null null null))
    (bind _output_get (set `self.CurrentCharge` (+ (`self.CurrentCharge`) (`self.deltaT`))))
    (`/Game/FirstPerson/Blueprints/BP_FirstPersonCharacter.OnChargeChanged` (`self.Owner`) (/ _output_get (`self.ChargeDuration`)))
    (if (`self.CanFire`)
      (`self.FireGun`))))

(fn `DamageHitEnemy`
  (params (Hit :type "HitResult Structure (by ref)"))
  (bind (_bblockinghit _binitialoverlap _time _distance _location _impactpoint _normal _impactnormal _physmat _hitactor) (`GameplayStatics.BreakHitResult` Hit))
  (`KismetSystemLibrary.PrintString` (`KismetSystemLibrary.GetDisplayName` _hitactor))
  (if (`GameplayStatics.ObjectIsA` _hitactor "/Game/JamContent/BPs/Pawns/BP_PBaseEnemy.BP_PBaseEnemy_C")
    (bind _returnvalue (`GameplayStatics.ApplyDamage` _hitactor (`self.Damage`) null (`self.GetOwner`)))
    (`KismetSystemLibrary.PrintString` (`KismetStringLibrary.Conv_DoubleToString` _returnvalue))))

(fn `FireGun`
  (bind _projectilelocation (`self.GetProjectileSpawnTransform`))
  (`GameplayStatics.PlaySound2D` (`self.FiringSound`) 0.5 1.0 0.0 null null)
  (bind _outhits (`KismetSystemLibrary.SphereTraceMultiForObjects` _projectilelocation (+ _projectilelocation (* (`Actor.GetActorForwardVector` (`GameplayStatics.GetPlayerCameraManager` 0)) 10000.0)) 7.0 (`self.Hittables`)))
  (for _array_element _outhits
    (`self.DamageHitEnemy` _array_element)
    (`self.SpawnSparksOnHit` _array_element))
  (`self.ReloadGun`)
  (`self.SpawnLaserParticle` (`self.GetProjectileSpawnTransform`) (`self.GetFinalImpactPoint` _outhits)))

(fn `SpawnLaserParticle`
  (params (Location :type "Vector Structure") (EndValue :type "Vector Structure"))
  (bind _returnvalue (`NiagaraFunctionLibrary.SpawnSystemAtLocation` "/Game/JamContent/Art/FX/NS_Laser.NS_Laser" Location))
  (`NiagaraComponent.SetVariableVec3` _returnvalue "LaserEndpoint" EndValue)
  (`NiagaraFunctionLibrary.SpawnSystemAtLocation` "/Game/JamContent/Art/FX/NS_LaserImpactSparks.NS_LaserImpactSparks" EndValue))

(fn `SpawnSparksOnHit`
  (params (Hit :type "HitResult Structure"))
  (`NiagaraFunctionLibrary.SpawnSystemAtLocation` "/Game/JamContent/Art/FX/NS_LaserImpactSparks.NS_LaserImpactSparks" (`.ImpactPoint` (`GameplayStatics.BreakHitResult` Hit))))