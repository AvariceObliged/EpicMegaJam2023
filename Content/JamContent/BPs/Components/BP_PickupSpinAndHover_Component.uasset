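; Pickup animation component that spins its owning actor, bobs it vertically, or does both, based on PickupType.
; BeginPlay caches the owner and its start location, then Tick applies yaw at SpinSpeed and sets position from a game-time sine wave.
; The hover lerp's alpha spans 0 to 2 rather than 0 to 1, so motion runs from HoverRange above the start to three times that below.
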(event `self.ReceiveBeginPlay`
  (bind _returnvalue (`self.GetOwner` self))
  (set `self.ParentActor` _returnvalue)
  (set `self.StartPosition` (`Actor.K2_GetActorLocation` _returnvalue)))

(event `self.ReceiveTick`
  (params (DeltaSeconds :type "Float (single-precision)"))
  (set `self.deltaT` DeltaSeconds)
  (switch `/Game/JamContent/BPs/Enumerations/PickupMovementType` (`self.PickupType`)
    (:`NewEnumerator1`
      (`self.Spin` (`self.deltaT`)))
    (:`NewEnumerator2`
      (`self.Hover`))
    (:`NewEnumerator3`
      (`self.Spin` (`self.deltaT`))
      (`self.Hover`))))

(fn `Hover`
  (locals (TopBounds :type "Vector Structure") (BottomBounds :type "Vector Structure"))
  (`Actor.K2_SetActorLocation` (`self.ParentActor`) (`KismetMathLibrary.VLerp` (+ (`self.StartPosition`) (`KismetMathLibrary.MakeVector` 0.0 0.0 (`self.HoverRange`))) (- (`self.StartPosition`) (`KismetMathLibrary.MakeVector` 0.0 0.0 (`self.HoverRange`))) (+ (`KismetMathLibrary.Sin` (* (+ (`KismetSystemLibrary.GetGameTimeInSeconds`) (`self.deltaT`)) (`self.HoverSpeed`))) 1.0)) false false))

(fn `Spin`
  (params (deltaT :type "Float (double-precision)"))
  (`Actor.K2_AddActorWorldRotation` (`self.ParentActor`) (`KismetMathLibrary.MakeRotator` 0.0 0.0 (* deltaT (`self.SpinSpeed`))) false false))