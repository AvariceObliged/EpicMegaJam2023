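; Actor component that spawns one batch of enemies along its owning BP_WavePathActor during a wave.
; BeginSpawning enables tick and seeds the timer so the first spawn follows the batch delay.
; Tick spawns through the path at each interval, carrying leftover time for catch-up spawns, then destroys the component once the count runs out.
; It increments the path's batch count on BeginPlay, and on EndPlay decrements it and asks the game mode to try ending the wave.
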(event `self.ReceiveBeginPlay`
  (bind _asbp_wave_path_actor (cast `/Game/JamContent/BPs/Actors/BP_WavePathActor` (`self.GetOwner`)))
  (bind _output_get (set `self.Path` _asbp_wave_path_actor))
  (set `/Game/JamContent/BPs/Actors/BP_WavePathActor.WaveBatchCount` (+ (`/Game/JamContent/BPs/Actors/BP_WavePathActor.WaveBatchCount` _output_get) 1) _output_get))

(event `Begin Spawning`
  (params (Batch :type "/Game/JamContent/BPs/Structs/WaveBatch Structure"))
  (`self.Initialize` Batch))

(event `self.ReceiveTick`
  (params (DeltaSeconds :type "Float (single-precision)"))
  (bind _returnvalue (> (`self.Remaining`) 0))
  (`self.IncrementTimer` DeltaSeconds)
  (while (and (`self.IsReadyToSpawn`) _returnvalue)
    (`self.Spawn`))
  (if (not _returnvalue)
    (`self.K2_DestroyComponent`)))

(event `self.ReceiveEndPlay`
  (params (EndPlayReason :type "EEndPlayReason Enum" :default "Destroyed"))
  (bind _path (`self.Path`))
  (set `/Game/JamContent/BPs/Actors/BP_WavePathActor.WaveBatchCount` (- (`/Game/JamContent/BPs/Actors/BP_WavePathActor.WaveBatchCount` _path) 1) _path)
  (`/Game/JamContent/BPs/BP_JamGameMode.TryEndWave` (`/Game/JamContent/BPs/Libraries/BP_Functions.GetJamGameMode`)))

(fn `IncrementTimer`
  (params (A :type "Float (double-precision)"))
  (set `self.Timer` (+ A (`self.Timer`))))

(fn `Initialize`
  (params (Batch :type "/Game/JamContent/BPs/Structs/WaveBatch Structure"))
  (bind (_enemy _interval _delay _count) (break `/Game/JamContent/BPs/Structs/WaveBatch` (`self.Batch`)))
  (set `self.Batch` Batch)
  (`self.SetComponentTickEnabled` true)
  (set `self.Timer` (- _interval _delay))
  (set `self.Remaining` _count))

(fn `IsReadyToSpawn`
  (returns (Ready :type Boolean))
  (return (> (`self.Timer`) (`.Interval_4_B6E5933F4194A1AEAADC408F6F587572` (break `/Game/JamContent/BPs/Structs/WaveBatch` (`self.Batch`))))))

(fn `Spawn`
  (bind (_enemy _interval) (break `/Game/JamContent/BPs/Structs/WaveBatch` (`self.Batch`)))
  (`/Game/JamContent/BPs/Actors/BP_WavePathActor.Spawn` (`self.Path`) _enemy)
  (set `self.Timer` (- (`self.Timer`) _interval))
  (set `self.Remaining` (- (`self.Remaining`) 1)))