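; Base gun component for the first-person character that attaches to the mesh's GripPoint socket and adds the weapon input mapping context.
; An AmmoType switch drives readiness, reload or cooldown timers and readouts for projectile and charge-up weapons, reported to the owner through change events.
; FireGun is an empty stub.
; Dropping can spawn the matching pickup actor by WeaponType, then clears the owner's weapon state and destroys the component.
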(event `self.ReceiveBeginPlay`
  (`self.InitializeGun`))

(event `EnhancedInput|/Game/FirstPerson/Input/Actions/IA_DropWeapon`
  (params (ActionValue :type Boolean) (ElapsedSeconds :type "Float (double-precision)") (TriggeredSeconds :type "Float (double-precision)") (InputAction :type "InputAction Object Reference" :default "/Game/FirstPerson/Input/Actions/IA_DropWeapon.IA_DropWeapon"))
  (:`Triggered`
    (`self.DropWeapon` true)))

(fn `CanFire`
  (returns (NewParam :type Boolean))
  (switch `/Game/JamContent/BPs/Enumerations/AmmoType` (`self.AmmoType`)
    (:`NewEnumerator0`
      (return (and (> (`self.CurrentAmmo`) 0) (`self.WeaponReady`))))
    (:`NewEnumerator1`
      (return (and (`self.WeaponReady`) (>= (`self.CurrentCharge`) (`self.ChargeDuration`)))))))

(fn `DropWeapon`
  (params (`Spawn Pickup` :type Boolean))
  (locals (DistanceFromPlayerToDropWeapon :type "Float (double-precision)" :default 100.0) (DropLocation :type "Transform Structure"))
  (bind _owner (`self.Owner`))
  (if `Spawn Pickup`
    (set `local.DropLocation` (`KismetMathLibrary.MakeTransform` (+ (* (`Actor.GetActorForwardVector` _owner) (`local.DistanceFromPlayerToDropWeapon`)) (`Actor.K2_GetActorLocation` _owner))))
    (switch `/Game/JamContent/BPs/Enumerations/WeaponType` (`self.WeaponType`)
      (:`NewEnumerator0`
        (`KismetSystemLibrary.PrintString` "Dropping 'None Weapon' with Left Beef"))
      (:`NewEnumerator1`
        (`|SpawnActorFromClass` "/Game/JamContent/BPs/Actors/BP_PickupGrenadeLauncher_Actor.BP_PickupGrenadeLauncher_Actor_C" (`local.DropLocation`) "Undefined" "MultiplyWithRoot" null null))
      (:`NewEnumerator2`
        (`|SpawnActorFromClass` "/Game/JamContent/BPs/Actors/BP_PickupMeltRifle_Actor.BP_PickupMeltRifle_Actor_C" (`local.DropLocation`) "Undefined" "MultiplyWithRoot" null null))
      (:`NewEnumerator3`
        (`|SpawnActorFromClass` "/Game/JamContent/BPs/Actors/BP_PickupSunderbuss_Actor.BP_PickupSunderbuss_Actor_C" (`local.DropLocation`) "Undefined" "MultiplyWithRoot" null null))))
  (bind _output_get (set `/Game/FirstPerson/Blueprints/BP_FirstPersonCharacter.EquippedWeaponType` "NewEnumerator0" (`self.Owner`)))
  (`/Game/FirstPerson/Blueprints/BP_FirstPersonCharacter.EquippedWeaponChanged` (`self.Owner`) _output_get)
  (`/Game/FirstPerson/Blueprints/BP_FirstPersonCharacter.OnReloadStateChanged` (`self.Owner`) false)
  (set `/Game/FirstPerson/Blueprints/BP_FirstPersonCharacter.HasWeapon` false (`self.Owner`))
  (bind _asplayer_controller (cast `PlayerController` (`Pawn.GetController` (`self.Owner`))))
  (`EnhancedInputSubsystemInterface.RemoveMappingContext` (pcsubsystem `EnhancedInputLocalPlayerSubsystem` _asplayer_controller) "/Game/FirstPerson/Input/IMC_Weapons.IMC_Weapons" (struct))
  (`self.K2_DestroyComponent`))

(fn `FireGun`)

(fn `GetAmmoReadout`
  (returns (ChargePercent :type "Float (double-precision)") (CurrentAmmo :type Integer) (MaxAmmo :type Integer))
  (switch `/Game/JamContent/BPs/Enumerations/AmmoType` (`self.AmmoType`)
    (:`NewEnumerator0`
      (return 0.0 (`self.CurrentAmmo`) (`self.MaxAmmo`)))
    (:`NewEnumerator1`
      (return (* (/ (`self.CurrentCharge`) (`self.ChargeDuration`)) 100.0) 0 0))))

(fn `GetProjectileSpawnTransform`
  (returns (ProjectileLocation :type "Vector Structure") (ProjectileRotator :type "Rotator Structure"))
  (bind _returnvalue (`PlayerCameraManager.GetCameraRotation` (`GameplayStatics.GetPlayerCameraManager` 0)))
  (return (+ (`self.GetSocketLocation` "Ammo") (`KismetMathLibrary.GreaterGreater_VectorRotator` (`self.ProjectileSpawnOffset`) _returnvalue)) _returnvalue))

(fn `InitializeGun`
  (bind _owner (`self.Owner`))
  (bind _asbp_first_person_character (cast `/Game/FirstPerson/Blueprints/BP_FirstPersonCharacter` (`self.GetOwner`)))
  (bind _output_get (set `self.Owner` _asbp_first_person_character))
  (`self.K2_AttachToComponent` (`/Game/FirstPerson/Blueprints/BP_FirstPersonCharacter.FirstPersonMesh` _output_get) "GripPoint" "SnapToTarget" "SnapToTarget" "SnapToTarget")
  (bind _asplayer_controller (cast `PlayerController` (`Pawn.GetController` (`self.Owner`))))
  (bind _returnvalue (pcsubsystem `EnhancedInputLocalPlayerSubsystem` _asplayer_controller))
  (`/Engine/EditorBlueprintResources/StandardMacros.IsValid` _returnvalue
    (:`Is Valid`
      (`EnhancedInputSubsystemInterface.AddMappingContext` _returnvalue "/Game/FirstPerson/Input/IMC_Weapons.IMC_Weapons" 1 (struct))
      (switch `/Game/JamContent/BPs/Enumerations/AmmoType` (`self.AmmoType`)
        (:`NewEnumerator0`
          (bind _output_get_2 (set `self.CurrentAmmo` (`self.MaxAmmo`)))
          (set `self.WeaponReady` true)
          (`/Game/FirstPerson/Blueprints/BP_FirstPersonCharacter.OnAmmoChanged` (`self.Owner`) _output_get_2))
        (:`NewEnumerator1`
          (bind _output_get_3 (set `self.CurrentCharge` 0.0))
          (set `self.WeaponReady` true)
          (`/Game/FirstPerson/Blueprints/BP_FirstPersonCharacter.OnChargeChanged` _owner _output_get_3)
          (`/Game/FirstPerson/Blueprints/BP_FirstPersonCharacter.OnChargeChanged` _owner 0.0))))))

(fn `MakeWeaponReady`
  (switch `/Game/JamContent/BPs/Enumerations/AmmoType` (`self.AmmoType`)
    (:`NewEnumerator0`
      (bind _output_get (set `self.CurrentAmmo` (`self.MaxAmmo`)))
      (`/Game/FirstPerson/Blueprints/BP_FirstPersonCharacter.OnAmmoChanged` (`self.Owner`) _output_get))
    (:`NewEnumerator1`
      _))
  (set `self.WeaponReady` true)
  (`/Game/FirstPerson/Blueprints/BP_FirstPersonCharacter.OnReloadStateChanged` (`self.Owner`) false))

(fn `PlayFireAnimation`
  (`AnimInstance.Montage_Play` (`self.GetAnimInstance` (`/Game/FirstPerson/Blueprints/BP_FirstPersonCharacter.FirstPersonMesh` (`self.Owner`))) (`self.FiringAnimation`) 1.0 "MontageLength" 0.0 true))

(fn `ReloadGun`
  (switch `/Game/JamContent/BPs/Enumerations/AmmoType` (`self.AmmoType`)
    (:`NewEnumerator0`
      (if (and (!= (`self.MaxAmmo`) (`self.CurrentAmmo`)) (`self.WeaponReady`))
        (set `self.WeaponReady` false) ; Mark Unready, begin reload process
        (`GameplayStatics.PlaySoundAtLocation` (`self.ReloadSound`) (`Actor.K2_GetActorLocation` (`self.Owner`)) (struct) 1.0 1.0 0.0 null null null null)
        (`KismetSystemLibrary.K2_SetTimer` null "MakeWeaponReady" (`self.ReloadDuration`))
        (`/Game/FirstPerson/Blueprints/BP_FirstPersonCharacter.OnReloadStateChanged` (`self.Owner`) true :!label _label)))
    (:`NewEnumerator1`
      (set `self.CurrentCharge` 0.0)
      (set `self.WeaponReady` false) ; Mark Unready, begin cooldown process
      (`KismetSystemLibrary.K2_SetTimer` null "MakeWeaponReady" (`self.CooldownDuration`))
      (goto _label))))