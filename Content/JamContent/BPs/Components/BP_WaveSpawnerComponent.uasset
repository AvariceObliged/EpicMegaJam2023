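; Wave spawner component for a BP_WavePathActor that releases a wave's enemy or unit batches in timed groups.
; BeginWave stores the wave and enables tick, which counts down each group's delay before passing all its batches to the owning path's SpawnBatch.
; After the last group it destroys itself, and EndPlay asks the game mode to TryEndWave.
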(event `self.ReceiveBeginPlay`
  (bind _asbp_wave_path_actor (cast `/Game/JamContent/BPs/Actors/BP_WavePathActor` (`self.GetOwner`)))
  (set `self.Path` _asbp_wave_path_actor))

(event `Begin Wave`
  (params (Wave :type "/Game/JamContent/BPs/Structs/Wave Structure"))
  (`self.Initialize` Wave))

(event `self.ReceiveTick`
  (params (DeltaSeconds :type "Float (single-precision)"))
  (`self.DecrementTimer` DeltaSeconds)
  (if (<= (`self.Timer`) 0.0)
    (`self.SpawnGroupBatches`)))

(event `self.ReceiveEndPlay`
  (params (EndPlayReason :type "EEndPlayReason Enum" :default "Destroyed"))
  (`/Game/JamContent/BPs/BP_JamGameMode.TryEndWave` (`/Game/JamContent/BPs/Libraries/BP_Functions.GetJamGameMode`)))

(fn `DecrementTimer`
  (params (InputPin :type "Float (single-precision)"))
  (set `self.Timer` (- (`self.Timer`) InputPin)))

(fn `GetCurrentGroup`
  (returns (Delay :type "Float (double-precision)") (Batches :type "Array of /Game/JamContent/BPs/Structs/WaveBatch Structure"))
  (bind (_delay _batches) (break `/Game/JamContent/BPs/Structs/WaveGroup` (`|GetArrayItem` (`.Groups_7_2228D65F479B921465CD1D83277A485D` (break `/Game/JamContent/BPs/Structs/Wave` (`self.Wave`))) (`self.CurrentGroupIndex`))))
  (return _delay _batches))

(fn `GetTimer`
  (returns (Timer :type "Float (double-precision)"))
  (return (`self.Timer`)))

(fn `Initialize`
  (params (Wave :type "/Game/JamContent/BPs/Structs/Wave Structure"))
  (set `self.Wave` Wave)
  (set `self.CurrentGroupIndex` 0)
  (`self.ResetTimer`)
  (`self.SetComponentTickEnabled` true))

(fn `ResetTimer`
  (set `self.Timer` (`self.GetCurrentGroup`)))

(fn `SpawnGroupBatches`
  (for _array_element (`.Batches` (`self.GetCurrentGroup`))
    (`/Game/JamContent/BPs/Actors/BP_WavePathActor.SpawnBatch` (`self.Path`) _array_element))
  (set `self.CurrentGroupIndex` (+ (`self.CurrentGroupIndex`) 1))
  (if (< (`self.CurrentGroupIndex`) (`KismetArrayLibrary.Array_Length` (`.Groups_7_2228D65F479B921465CD1D83277A485D` (break `/Game/JamContent/BPs/Structs/Wave` (`self.Wave`)))))
    (`self.ResetTimer`)
    (else
      (`self.K2_DestroyComponent`))))