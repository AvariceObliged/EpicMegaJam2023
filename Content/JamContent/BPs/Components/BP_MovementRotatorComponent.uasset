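; Actor component that turns its owning actor to face roughly along its horizontal movement.
; On begin play it caches the owner's FloatingPawnMovement and ticks only if one exists.
; Each tick, while planar velocity is non-zero, it snaps the owner's rotation without interpolation.
; The rotation is a look-at from the constant world forward vector to the velocity vector, so it deviates slightly from the true heading.
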(event `self.ReceiveBeginPlay`
  (bind _output_get (set `self.PawnMovement` (`Actor.GetComponentByClass` (`self.GetOwner`) "/Script/Engine.FloatingPawnMovement")))
  (`self.SetComponentTickEnabled` (`KismetSystemLibrary.IsValid` _output_get)))

(event `self.ReceiveTick`
  (params (DeltaSeconds :type "Float (single-precision)"))
  (bind _returnvalue (`KismetMathLibrary.MakeVector` (.x (`MovementComponent.Velocity` (`self.PawnMovement`))) (.y (`MovementComponent.Velocity` (`self.PawnMovement`)))))
  (if (not (`KismetMathLibrary.Vector_IsNearlyZero` _returnvalue))
    (`Actor.K2_SetActorRotation` (`self.GetOwner`) (`KismetMathLibrary.FindLookAtRotation` (`KismetMathLibrary.Vector_Forward`) _returnvalue) false)))