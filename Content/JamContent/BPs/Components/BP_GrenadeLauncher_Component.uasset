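; Grenade launcher weapon component that fires projectiles and reloads in response to the Enhanced Input shoot and reload actions.
; Shooting is gated by CanFire, then FireGun decrements ammo, spawns the projectile actor at the computed spawn transform, and plays the firing sound and animation.
; Each shot reports the new ammo count to the owner through its OnAmmoChanged dispatcher.
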(event `EnhancedInput|/Game/FirstPerson/Input/Actions/IA_Shoot`
  (params (ActionValue :type Boolean) (ElapsedSeconds :type "Float (double-precision)") (TriggeredSeconds :type "Float (double-precision)") (InputAction :type "InputAction Object Reference" :default "/Game/FirstPerson/Input/Actions/IA_Shoot.IA_Shoot"))
  (:`Triggered`
    (if (`self.CanFire`)
      (`self.FireGun`))))

(event `EnhancedInput|/Game/FirstPerson/Input/Actions/IA_Reload`
  (params (ActionValue :type Boolean) (ElapsedSeconds :type "Float (double-precision)") (TriggeredSeconds :type "Float (double-precision)") (InputAction :type "InputAction Object Reference" :default "/Game/FirstPerson/Input/Actions/IA_Reload.IA_Reload"))
  (:`Triggered`
    (`self.ReloadGun`)))

(fn `CreateProjectile`
  (params (Location :type "Vector Structure") (Rotation :type "Rotator Structure"))
  (`|SpawnActorFromClass` (`self.Projectile`) (`KismetMathLibrary.MakeTransform` Location Rotation) "Undefined" "OverrideRootScale" null null))

(fn `FireGun`
  (bind (_projectilelocation _projectilerotator) (`self.GetProjectileSpawnTransform`))
  (`/Engine/EditorBlueprintResources/StandardMacros.DecrementInt` (`self.CurrentAmmo`)
    (:`  `
      (`self.CreateProjectile` _projectilelocation _projectilerotator)
      (`GameplayStatics.PlaySound2D` (`self.FiringSound`) 1.0 1.0 0.0 null null)
      (`self.PlayFireAnimation`)
      (`/Game/FirstPerson/Blueprints/BP_FirstPersonCharacter.OnAmmoChanged` (`self.Owner`) (`self.CurrentAmmo`)))))