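; BP_EnemyHealthComponent is an enemy health component that tracks current health against a maximum.
; Current health starts at the maximum on BeginPlay, and ApplyDamage subtracts from it, destroying the owning actor once it reaches zero or below.
; GetRatio returns current health as a fraction of maximum health.
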(event `self.ReceiveBeginPlay`
  (set `self.CurrentHealth` (`self.MaxHealth`)))

(fn `ApplyDamage`
  (params (Damage :type "Float (double-precision)"))
  (bind _output_get (set `self.CurrentHealth` (- (`self.CurrentHealth`) Damage)))
  (if (<= _output_get 0.0)
    (`Actor.K2_DestroyActor` (`self.GetOwner`))))

(fn `GetRatio`
  (returns (HealthRatio :type "Float (double-precision)"))
  (return (/ (`self.CurrentHealth`) (`self.MaxHealth`))))