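; Sunderbuss shotgun component that fires and reloads the weapon from Enhanced Input shoot and reload actions.
; Each shot spends one ammo and spawns two pellet bursts, an inner and an outer cone, each with its own count and spread angle.
; Pellets are projectile actors launched in random directions within their cone from the projectile spawn transform, accompanied by pooled Niagara sparks and a fire animation.
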(event `EnhancedInput|/Game/FirstPerson/Input/Actions/IA_Shoot`
  (params (ActionValue :type Boolean) (ElapsedSeconds :type "Float (double-precision)") (TriggeredSeconds :type "Float (double-precision)") (InputAction :type "InputAction Object Reference" :default "/Game/FirstPerson/Input/Actions/IA_Shoot.IA_Shoot"))
  (:`Triggered`
    (if (`self.CanFire`)
      (`self.FireGun`))))

(event `EnhancedInput|/Game/FirstPerson/Input/Actions/IA_Reload`
  (params (ActionValue :type Boolean) (ElapsedSeconds :type "Float (double-precision)") (TriggeredSeconds :type "Float (double-precision)") (InputAction :type "InputAction Object Reference" :default "/Game/FirstPerson/Input/Actions/IA_Reload.IA_Reload"))
  (:`Triggered`
    (`self.ReloadGun`)))

(fn `FireGun`
  (`/Engine/EditorBlueprintResources/StandardMacros.DecrementInt` (`self.CurrentAmmo`)
    (:`  `
      (`self.FireProjectileBurst` (`self.PelletsPerShotInner`) (`self.VarianceAngleInner`)) ; Fire Inner Burst
      (`self.FireProjectileBurst` (`self.PelletsPerShotOuter`) (`self.VarianceAngleOuter`)) ; Fire Outer Burst
      (`NiagaraFunctionLibrary.SpawnSystemAtLocation` "/Game/JamContent/Art/FX/NS_SunderbussSparks.NS_SunderbussSparks" (0.0 0.0 0.0) (struct) (1.0 1.0 1.0) true true "AutoRelease")
      (`self.PlayFireAnimation`))))

(fn `FireProjectileBurst`
  (params (`Shot Count` :type Integer) (Variance :type "Float (double-precision)"))
  (for _ (range 1 (+ `Shot Count` 1))
    (`self.FireSingleProjectile` Variance)))

(fn `FireSingleProjectile`
  (params (Variance :type "Float (double-precision)"))
  (bind (_projectilelocation _projectilerotator) (`self.GetProjectileSpawnTransform`))
  (bind _owner (`self.Owner`))
  (`|SpawnActorFromClass` (`self.Projectile`) (`KismetMathLibrary.MakeTransform` _projectilelocation (`KismetMathLibrary.Conv_VectorToRotator` (`KismetMathLibrary.RandomUnitVectorInConeInDegrees` (`KismetMathLibrary.Conv_RotatorToVector` _projectilerotator) Variance))) "AlwaysSpawn" "OverrideRootScale" _owner _owner))

(fn `ReloadingComplete`)