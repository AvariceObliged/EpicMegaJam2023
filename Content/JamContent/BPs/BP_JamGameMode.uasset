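; Game mode that runs a wave-based enemy level and creates the HUD on begin play.
; It gathers all BP_WavePathActor instances, takes the largest wave count among them, and starts waves from Tick whenever none is active.
; Enemies are tracked in a list, and TryEndWave advances once none remain and no path is spawning.
; After the last wave, it opens the level referenced by the BP_NextLevel actor.
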(event `self.ReceiveBeginPlay`
  (`self.FindWavePaths`)
  (bind _returnvalue (`|CreateWidget` "/Game/JamContent/BPs/BP_HUDWidget.BP_HUDWidget_C"))
  (`UserWidget.AddToViewport` _returnvalue 0))

(event `self.ReceiveTick`
  (params (DeltaSeconds :type "Float (single-precision)"))
  (`self.StartWave`))

(fn `AnyActivelySpawningWaves`
  (returns (Result :type Boolean))
  (for _array_element (`self.WavePaths`)
    (if (`/Game/JamContent/BPs/Actors/BP_WavePathActor.IsActivelySpawning` _array_element)
      (return true)))
  (return false))

(fn `FindWavePaths`
  (bind _outactors (`GameplayStatics.GetAllActorsOfClass` "/Game/JamContent/BPs/Actors/BP_WavePathActor.BP_WavePathActor_C"))
  (bind _output_get (set `self.WavePaths` _outactors))
  (for _array_element _output_get
    (set `self.WaveCount` (`KismetMathLibrary.Max` (`/Game/JamContent/BPs/Actors/BP_WavePathActor.GetWaveCount` _array_element) (`self.WaveCount`)))))

(fn `Get Wave Number`
  (returns (WaveNumber :type Integer))
  (return (+ (`self.WaveIndex`) 1)))

(fn `GetTrackedEnemyCount`
  (returns (Count :type Integer))
  (return (`BlueprintSetLibrary.Set_Length` (`self.TrackedEnemies`))))

(fn `HasTrackedEnemies`
  (returns (Result :type Boolean))
  (return (> (`self.GetTrackedEnemyCount`) 0)))

(fn `StartWave`
  (if (and (not (`self.IsWaveActive`)) (< (`self.WaveIndex`) (`self.WaveCount`)))
    (set `self.IsWaveActive` true)
    (`self.WaveStart` (`self.WaveIndex`))))

(fn `TrackEnemy`
  (params (Enemy :type "Pawn Object Reference"))
  (`BlueprintSetLibrary.Set_Add` (`self.TrackedEnemies`) Enemy))

(fn `TryEndWave`
  (if (and (`self.IsWaveActive`) (`KismetMathLibrary.BooleanNOR` (`self.HasTrackedEnemies`) (`self.AnyActivelySpawningWaves`)))
    (set `self.IsWaveActive` false)
    (set `self.WaveIndex` (+ (`self.WaveIndex`) 1))
    (if (< (`self.WaveIndex`) (`self.WaveCount`))
      (`self.WaveEnd`)
      (else
        (bind _returnvalue (`GameplayStatics.GetActorOfClass` "/Game/JamContent/BPs/Actors/BP_NextLevel.BP_NextLevel_C"))
        (`GameplayStatics.OpenLevelBySoftObjectPtr` (`/Game/JamContent/BPs/Actors/BP_NextLevel.Value` _returnvalue))))))

(fn `UntrackEnemy`
  (params (Enemy :type "Pawn Object Reference (by ref)"))
  (`BlueprintSetLibrary.Set_Remove` (`self.TrackedEnemies`) Enemy))

(fn `UserConstructionScript`)