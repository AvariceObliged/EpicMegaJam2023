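; BP_SunderbussProjectile_Actor is the Sunderbuss's ricocheting projectile, which damages enemies and expires after a set lifetime or bounce count.
; All hit logic runs on ProjectileMovement's bounce event: hitting a BP_PBaseEnemy applies damage, prints the enemy's name and destroys the projectile.
; Other impacts increment a bounce counter and spawn a pooled Niagara ricochet effect until the limit destroys it.
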(event `self.ReceiveBeginPlay`
  (`KismetSystemLibrary.K2_SetTimer` null "DestroySelf" (`self.ProjectileLifetime`)))

(event `self.ProjectileMovement.OnProjectileBounce`
  (params (ImpactResult :type "HitResult Structure (by ref)") (ImpactVelocity :type "Vector Structure (by ref)"))
  (if (`GameplayStatics.ObjectIsA` ImpactResult_HitActor "/Game/JamContent/BPs/Pawns/BP_PBaseEnemy.BP_PBaseEnemy_C")
    (`GameplayStatics.ApplyDamage` ImpactResult_HitActor (`self.ProjectileDamage`))
    (`KismetSystemLibrary.PrintString` (`KismetSystemLibrary.GetDisplayName` ImpactResult_HitActor))
    (`self.DestroySelf`)
    (else
      (bind _result (`/Engine/EditorBlueprintResources/StandardMacros.IncrementInt` (`self.Bounces`))
        (:`  `
          (if (>= _result (`self.MaxBounces`))
            (`self.DestroySelf`)
            (else
              (`NiagaraFunctionLibrary.SpawnSystemAtLocation` "/Game/JamContent/Art/FX/NS_SunderbussRicochet.NS_SunderbussRicochet" ImpactResult_Location (struct) (1.0 1.0 1.0) true true "AutoRelease"))))))))

(fn `DestroySelf`
  (`self.K2_DestroyActor`))

(fn `UserConstructionScript`)