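; Weapon tower that automatically fires at enemies with whichever weapon the player trades into it.
; The player's trade event gives, takes or swaps weapons while inside GiveTrigger.
; SetTowerWeapon sets the mesh, targeting radius and looping fire timer for each weapon type.
; Each shot aims at the closest line-of-sight enemy, then spawns grenade or spread Sunderbuss projectiles, or a damaging Melt Rifle sphere-trace laser.
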(event `self.ReceiveBeginPlay`
  (`self.InitializeTower`)
  (bind _returnvalue (`GameplayStatics.GetActorOfClass` "/Game/FirstPerson/Blueprints/BP_FirstPersonCharacter.BP_FirstPersonCharacter_C"))
  (add `/Game/FirstPerson/Blueprints/BP_FirstPersonCharacter.AttemptTradeWeapon` _returnvalue (delegate `StartTradeAttempt`)))

(event `StartTradeAttempt`
  (`KismetSystemLibrary.PrintString` "Trade weapon triggered")
  (if (`self.IsPlayerInRangeToTrade`)
    (`self.HandleTradeAttempt`)
    (else
      (`KismetSystemLibrary.PrintString` "Player out of range"))))

(event `self.GiveTrigger.OnComponentBeginOverlap`
  (params (OverlappedComponent :type "PrimitiveComponent Object Reference") (OtherActor :type "Actor Object Reference") (OtherComp :type "PrimitiveComponent Object Reference") (OtherBodyIndex :type Integer) (bFromSweep :type Boolean) (SweepResult :type "HitResult Structure (by ref)"))
  (bind _asbp_first_person_character (cast `/Game/FirstPerson/Blueprints/BP_FirstPersonCharacter` OtherActor))
  (`self.PlayerEnteredTradeRange` (`self.TowerWeaponType`) (`/Game/FirstPerson/Blueprints/BP_FirstPersonCharacter.EquippedWeaponType` _asbp_first_person_character)))

(event `self.GiveTrigger.OnComponentEndOverlap`
  (params (OverlappedComponent :type "PrimitiveComponent Object Reference") (OtherActor :type "Actor Object Reference") (OtherComp :type "PrimitiveComponent Object Reference") (OtherBodyIndex :type Integer))
  (cast `/Game/FirstPerson/Blueprints/BP_FirstPersonCharacter` OtherActor)
  (`self.PlayerExitedTradeRange`))

(fn `AimTowerAtTarget`
  (params (`Actor to aim at` :type "Actor Object Reference"))
  (bind _turret (`self.Turret`))
  (`SceneComponent.K2_SetWorldRotation` _turret (`KismetMathLibrary.FindLookAtRotation` (`SceneComponent.K2_GetComponentLocation` _turret) (`self.K2_GetActorLocation` `Actor to aim at`)) false false))

(fn `FireTowerWeapon`
  (if (`self.TowerHasWeapon`)
    (bind (_closestvalidtarget _hasvalidtarget) (`self.GetClosestValidTarget` (`self.GetEnemiesInRange`)))
    (if _hasvalidtarget
      (`self.AimTowerAtTarget` _closestvalidtarget)
      (switch `/Game/JamContent/BPs/Enumerations/WeaponType` (`self.TowerWeaponType`)
        (:`NewEnumerator1`
          (`self.CreateProjectile` "/Game/JamContent/BPs/Actors/BP_GrenadeLauncherProjectile_Actor.BP_GrenadeLauncherProjectile_Actor_C" 1
            (:`Completed`
              (`GameplayStatics.PlaySoundAtLocation` "/Game/JamContent/Art/Audio/SFX/Temp/grenadeShot.grenadeShot" (`SceneComponent.K2_GetComponentLocation` (`self.Turret`)) (struct) 1.0 1.0 0.0 null null null null))))
        (:`NewEnumerator2`
          (`self.CreateLaserSpherecast`
            (:`Output`
              (`GameplayStatics.PlaySoundAtLocation` "/Game/JamContent/Art/Audio/SFX/Temp/pew.pew" (`SceneComponent.K2_GetComponentLocation` (`self.Turret`)) (struct) 0.5 1.0 0.0 null null null null))))
        (:`NewEnumerator3`
          (`self.CreateProjectile` "/Game/JamContent/BPs/Actors/BP_SunderbussProjectile_Actor.BP_SunderbussProjectile_Actor_C" 4 2.0
            (:`Completed`
              (`self.CreateProjectile` "/Game/JamContent/BPs/Actors/BP_SunderbussProjectile_Actor.BP_SunderbussProjectile_Actor_C" 6 4.0
                (:`Completed`
                  (`GameplayStatics.PlaySoundAtLocation` "/Game/JamContent/Art/Audio/SFX/Temp/sunderbuss.sunderbuss" (`SceneComponent.K2_GetComponentLocation` (`self.Turret`)) (struct) 0.5 1.0 0.0 null null null null)))))))
      (else
        (`KismetSystemLibrary.PrintString` "No valid targets")))))

(fn `GetClosestValidTarget`
  (params (TargetsInRange :type "Array of Actor Object Reference"))
  (returns (ClosestValidTarget :type "Actor Object Reference") (HasValidTarget :type Boolean))
  (locals (CurrentClosestTarget :type "Actor Object Reference") (ValidTargets :type "Map of Actor Object Reference to Float (double-precision)") (CurrentElement :type "Actor Object Reference"))
  (for _array_element TargetsInRange
    (set `local.CurrentElement` _array_element)
    (bind _outhit (`KismetSystemLibrary.LineTraceSingleForObjects` (`SceneComponent.K2_GetComponentLocation` (`self.Turret`)) (`self.K2_GetActorLocation` (`local.CurrentElement`)) (`self.RaycastObjectTypes`)))
    (bind (_bblockinghit _binitialoverlap _time _distance _location _impactpoint _normal _impactnormal _physmat _hitactor) (`GameplayStatics.BreakHitResult` _outhit))
    (if (`GameplayStatics.ObjectIsA` _hitactor "/Game/JamContent/BPs/Pawns/BP_PBaseEnemy.BP_PBaseEnemy_C")
      (`BlueprintMapLibrary.Map_Add` (`local.ValidTargets`) (`local.CurrentElement`) _distance)
      (set `local.CurrentClosestTarget` (`local.CurrentElement`)) ; Just sets the most recent valid so we have a placeholder so this is never null
    ))
  (if (> (`BlueprintMapLibrary.Map_Length` (`local.ValidTargets`)) 0)
    (bind _keys (`BlueprintMapLibrary.Map_Keys` (`local.ValidTargets`)))
    (for _array_element_2 _keys
      (set `local.CurrentElement` _array_element_2)
      (if (< (`BlueprintMapLibrary.Map_Find` (`local.ValidTargets`) (`local.CurrentElement`)) (`BlueprintMapLibrary.Map_Find` (`local.ValidTargets`) (`local.CurrentClosestTarget`)))
        (set `local.CurrentClosestTarget` (`local.CurrentElement`))))
    (return (`local.CurrentClosestTarget`) true)
    (else
      (`KismetSystemLibrary.PrintString` "No targets visible")
      (return null false))))

(fn `HandleGiveToTower`
  (params (CharacterReference :type "/Game/FirstPerson/Blueprints/BP_FirstPersonCharacter Object Reference"))
  (locals (PlayerWeaponType :type "/Game/JamContent/BPs/Enumerations/WeaponType Enum"))
  (bind _equippedweapontype (`/Game/FirstPerson/Blueprints/BP_FirstPersonCharacter.EquippedWeaponType` CharacterReference))
  (`KismetSystemLibrary.PrintString` "Attempting to give weapon to tower")
  (`self.SetTowerWeapon` _equippedweapontype)
  (switch `/Game/JamContent/BPs/Enumerations/WeaponType` _equippedweapontype
    (:`NewEnumerator1`
      (`/Game/JamContent/BPs/Components/BP_GunComponent_Base.DropWeapon` (`self.GetComponentByClass` (`local.CharacterReference`) "/Game/JamContent/BPs/Components/BP_GrenadeLauncher_Component.BP_GrenadeLauncher_Component_C") false))
    (:`NewEnumerator2`
      (`/Game/JamContent/BPs/Components/BP_GunComponent_Base.DropWeapon` (`self.GetComponentByClass` (`local.CharacterReference`) "/Game/JamContent/BPs/Components/BP_MeltRifle_Component.BP_MeltRifle_Component_C") false))
    (:`NewEnumerator3`
      (`/Game/JamContent/BPs/Components/BP_GunComponent_Base.DropWeapon` (`self.GetComponentByClass` (`local.CharacterReference`) "/Game/JamContent/BPs/Components/BP_Sunderbuss_Component.BP_Sunderbuss_Component_C") false))))

(fn `HandleSwapWithTower`
  (params (CharacterReference :type "/Game/FirstPerson/Blueprints/BP_FirstPersonCharacter Object Reference"))
  (locals (PlayerWeaponType :type "/Game/JamContent/BPs/Enumerations/WeaponType Enum" :default "NewEnumerator0"))
  (bind _characterreference (`local.CharacterReference`))
  (`KismetSystemLibrary.PrintString` "Attempting weapon swap")
  (bind _output_get (set `local.PlayerWeaponType` (`/Game/FirstPerson/Blueprints/BP_FirstPersonCharacter.EquippedWeaponType` CharacterReference)))
  (switch `/Game/JamContent/BPs/Enumerations/WeaponType` _output_get
    (:`NewEnumerator0`
      (`KismetSystemLibrary.PrintString` "ERROR Player weapon type None"))
    (:`NewEnumerator1`
      (`/Game/JamContent/BPs/Components/BP_GunComponent_Base.DropWeapon` (`self.GetComponentByClass` (`local.CharacterReference`) "/Game/JamContent/BPs/Components/BP_GrenadeLauncher_Component.BP_GrenadeLauncher_Component_C") false)
      (switch `/Game/JamContent/BPs/Enumerations/WeaponType` (`self.TowerWeaponType`) :!label _label
        (:`NewEnumerator0`
          (`KismetSystemLibrary.PrintString` "ERROR: Tower weapon type NONE"))
        (:`NewEnumerator1`
          (`AddComponent|NODE_AddBP_GrenadeLauncher_Component-0` :`self` _characterreference)
          (set `/Game/FirstPerson/Blueprints/BP_FirstPersonCharacter.EquippedWeaponType` (`self.TowerWeaponType`) (`local.CharacterReference`) :!label _label_2)
          (set `/Game/FirstPerson/Blueprints/BP_FirstPersonCharacter.HasWeapon` true (`local.CharacterReference`))
          (`self.SetTowerWeapon` (`local.PlayerWeaponType`)))
        (:`NewEnumerator2`
          (`AddComponent|NODE_AddBP_MeltRifle_Component-0` :`self` _characterreference)
          (goto _label_2))
        (:`NewEnumerator3`
          (`AddComponent|NODE_AddBP_Sunderbuss_Component-0` :`self` _characterreference)
          (goto _label_2))))
    (:`NewEnumerator2`
      (`/Game/JamContent/BPs/Components/BP_GunComponent_Base.DropWeapon` (`self.GetComponentByClass` (`local.CharacterReference`) "/Game/JamContent/BPs/Components/BP_MeltRifle_Component.BP_MeltRifle_Component_C") false)
      (goto _label))
    (:`NewEnumerator3`
      (`/Game/JamContent/BPs/Components/BP_GunComponent_Base.DropWeapon` (`self.GetComponentByClass` (`local.CharacterReference`) "/Game/JamContent/BPs/Components/BP_Sunderbuss_Component.BP_Sunderbuss_Component_C") false)
      (goto _label))))

(fn `HandleTakeFromTower`
  (params (CharacterReference :type "/Game/FirstPerson/Blueprints/BP_FirstPersonCharacter Object Reference"))
  (`KismetSystemLibrary.PrintString` "Attempting take weapon from tower")
  (switch `/Game/JamContent/BPs/Enumerations/WeaponType` (`self.TowerWeaponType`)
    (:`NewEnumerator1`
      (`AddComponent|NODE_AddBP_GrenadeLauncher_Component-1` :`self` (`local.CharacterReference`)))
    (:`NewEnumerator2`
      (`AddComponent|NODE_AddBP_MeltRifle_Component-1` :`self` (`local.CharacterReference`)))
    (:`NewEnumerator3`
      (`AddComponent|NODE_AddBP_Sunderbuss_Component-1` :`self` (`local.CharacterReference`))))
  (set `/Game/FirstPerson/Blueprints/BP_FirstPersonCharacter.HasWeapon` true (`local.CharacterReference`))
  (set `/Game/FirstPerson/Blueprints/BP_FirstPersonCharacter.EquippedWeaponType` (`self.TowerWeaponType`) (`local.CharacterReference`))
  (`self.SetTowerWeapon` "NewEnumerator0"))

(fn `HandleTradeAttempt`
  (locals (LocalFirstPersonCharacter :type "/Game/FirstPerson/Blueprints/BP_FirstPersonCharacter Object Reference"))
  (bind _localfirstpersoncharacter (`local.LocalFirstPersonCharacter`))
  (bind _asbp_first_person_character (cast `/Game/FirstPerson/Blueprints/BP_FirstPersonCharacter` (`|GetArrayItem` (`PrimitiveComponent.GetOverlappingActors` (`self.GiveTrigger`) "/Game/FirstPerson/Blueprints/BP_FirstPersonCharacter.BP_FirstPersonCharacter_C"))))
  (bind _output_get (set `local.LocalFirstPersonCharacter` _asbp_first_person_character))
  (if (and (`/Game/FirstPerson/Blueprints/BP_FirstPersonCharacter.HasWeapon` _output_get) (`self.TowerHasWeapon`))
    (if (`self.TowerHasWeapon`)
      (`self.HandleSwapWithTower` _localfirstpersoncharacter)
      (`self.PlayerEnteredTradeRange` (`self.TowerWeaponType`) (`/Game/FirstPerson/Blueprints/BP_FirstPersonCharacter.EquippedWeaponType` (`local.LocalFirstPersonCharacter`)) :!label _label))
    (elif (`self.TowerHasWeapon`)
      (`self.HandleTakeFromTower` _localfirstpersoncharacter)
      (goto _label)
      (else
        (`self.HandleGiveToTower` _localfirstpersoncharacter)
        (goto _label)))))

(fn `InitializeTower`
  (`self.SetTowerWeapon` (`self.TowerWeaponType`)))

(fn `SetTowerWeapon`
  (params (NewWeaponType :type "/Game/JamContent/BPs/Enumerations/WeaponType Enum" :default "NewEnumerator0"))
  (bind _output_get (set `self.TowerWeaponType` NewWeaponType))
  (`KismetSystemLibrary.K2_ClearTimer` null "FireTowerWeapon")
  (switch `/Game/JamContent/BPs/Enumerations/WeaponType` _output_get
    (:`NewEnumerator0`
      ;[1 1 1] No Weapon
      (`SphereComponent.SetSphereRadius` (`self.TargetingTrigger`) 0.0 true)
      (`SceneComponent.SetVisibility` (`self.TurretDisplayMesh`) false false)
      (set `self.TowerHasWeapon` false))
    (:`NewEnumerator1`
      ;[1 0.871 0.3434] Set to Grenade Launcher
      (`SphereComponent.SetSphereRadius` (`self.TargetingTrigger`) (`self.TowerRangeGrenadeLauncher`) true)
      (set `SkeletalMeshComponent.SkeletalMeshAsset` (`self.GrenadeLauncherMesh`) (`self.TurretDisplayMesh`))
      (`KismetSystemLibrary.K2_SetTimer` null "FireTowerWeapon" (`self.TimeBetweenShotsGrenadeLauncher`) true)
      (`SceneComponent.SetVisibility` (`self.TurretDisplayMesh`) true false :!label _label)
      (set `self.TowerHasWeapon` true))
    (:`NewEnumerator2`
      ;[0.3785 0.8594 1] Set to Melt Rifle
      (`SphereComponent.SetSphereRadius` (`self.TargetingTrigger`) (`self.TowerRangeMeltRifle`) true)
      (set `SkeletalMeshComponent.SkeletalMeshAsset` (`self.MeltRifleMesh`) (`self.TurretDisplayMesh`))
      (`KismetSystemLibrary.K2_SetTimer` null "FireTowerWeapon" (`self.TimeBetweenShotsMeltRifle`) true)
      (goto _label))
    (:`NewEnumerator3`
      ;[1 0.2511 0.1614] Set to Sunderbuss
      (`SphereComponent.SetSphereRadius` (`self.TargetingTrigger`) (`self.TowerRangeSunderbuss`) true)
      (set `SkeletalMeshComponent.SkeletalMeshAsset` (`self.SunderbussMesh`) (`self.TurretDisplayMesh`))
      (`KismetSystemLibrary.K2_SetTimer` null "FireTowerWeapon" (`self.TimeBetweenShotsSunderbuss`) true)
      (goto _label))))

(fn `UserConstructionScript`)