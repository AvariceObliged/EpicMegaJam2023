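; BP_Pickup_Gun_Base is a gun pickup actor that arms a first-person character who overlaps its collision sphere.
; The overlap runs DoPickup, which accepts only a BP_FirstPersonCharacter without a weapon and copies the pickup's WeaponType to it.
; AssignEquippedMesh then adds a BP weapon component to the character, and the pickup destroys itself.
; Characters that already have a weapon only trigger a debug print.
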(event `self.SphereCollision.OnComponentBeginOverlap`
  (params (OverlappedComponent :type "PrimitiveComponent Object Reference") (OtherActor :type "Actor Object Reference") (OtherComp :type "PrimitiveComponent Object Reference") (OtherBodyIndex :type Integer) (bFromSweep :type Boolean) (SweepResult :type "HitResult Structure (by ref)"))
  (`self.DoPickup` OtherActor))

(fn `AssignEquippedMesh`
  (params (CharacterReference :type "/Game/FirstPerson/Blueprints/BP_FirstPersonCharacter Object Reference"))
  (`AddComponent|NODE_AddBP_Weapon_Component-2` :`self` CharacterReference))

(fn `DestroySelf`
  (`self.K2_DestroyActor`))

(fn `DoPickup`
  (params (`Other Actor` :type "Object Object Reference"))
  (locals (Local_FPSCharacter :type "/Game/FirstPerson/Blueprints/BP_FirstPersonCharacter Object Reference"))
  (if (`GameplayStatics.ObjectIsA` `Other Actor` "/Game/FirstPerson/Blueprints/BP_FirstPersonCharacter.BP_FirstPersonCharacter_C")
    (bind _asbp_first_person_character (cast `/Game/FirstPerson/Blueprints/BP_FirstPersonCharacter` (`local.Other Actor`))
      (:`then`
        (bind _output_get (set `local.Local_FPSCharacter` _asbp_first_person_character))
        (if (`/Game/FirstPerson/Blueprints/BP_FirstPersonCharacter.HasWeapon` _output_get)
          (`KismetSystemLibrary.PrintString` "ACTOR HAS WEAPON ALREADY")
          (else
            (set `/Game/FirstPerson/Blueprints/BP_FirstPersonCharacter.HasWeapon` true (`local.Local_FPSCharacter`))
            (set `/Game/FirstPerson/Blueprints/BP_FirstPersonCharacter.EquippedWeaponType` (`self.WeaponType`) (`local.Local_FPSCharacter`))
            (`self.AssignEquippedMesh` (`local.Local_FPSCharacter`))
            (`self.DestroySelf`))))
      (:`CastFailed`
        (`KismetSystemLibrary.PrintString` "Cast to BP_FirstPersonCharacter FAILED")))))

(fn `UserConstructionScript`)