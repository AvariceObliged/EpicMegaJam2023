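; Wave path actor that spawns enemies at its own transform and supplies an ordered list of waypoints for their route.
; BeginPlay starts a hardcoded three-group wave of Walter test pawns through a dynamically added wave spawner component; batches get their own spawner components.
; Spawn hands the path to each enemy's BP_WavePathingComponent.
; VisualizePath draws navmesh paths from the actor through the waypoints as temporary debug lines.
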(event `self.ReceiveBeginPlay`
  (bind _array (`|MakeArray` (make `/Game/JamContent/BPs/Structs/WaveBatch` "/Game/JamContent/BPs/Pawns/BP_WalterTestPawn.BP_WalterTestPawn_C" 0.3 3.0 15) (make `/Game/JamContent/BPs/Structs/WaveBatch` "/Game/JamContent/BPs/Pawns/BP_WalterTestPawn2.BP_WalterTestPawn2_C" 0.7 0.0 6)))
  (bind _wavegroup (make `/Game/JamContent/BPs/Structs/WaveGroup` 10.0 _array))
  (`self.SpawnWave` (make `/Game/JamContent/BPs/Structs/Wave` (`|MakeArray` (make `/Game/JamContent/BPs/Structs/WaveGroup` 3.0 _array) _wavegroup _wavegroup))))

(fn `DrawPathSegment`
  (params (Start :type "Vector Structure") (End :type "Vector Structure"))
  (bind _returnvalue (* (`KismetMathLibrary.Vector_Up`) 100))
  (bind _returnvalue_2 (`NavigationSystemV1.FindPathToLocationSynchronously` Start End null null))
  (bind _pathpoints (`NavigationPath.PathPoints` _returnvalue_2))
  (for _index (range (+ (- (`KismetArrayLibrary.Array_Length` _pathpoints) 2) 1))
    (`KismetSystemLibrary.DrawDebugLine` (+ (`|GetArrayItem` _pathpoints _index) _returnvalue) (+ (`|GetArrayItem` _pathpoints (+ _index 1)) _returnvalue) (struct :`R` 1.0 :`A` 1.0) 2.0 20.0)))

(fn `GetWaypointCount`
  (returns (Count :type Integer))
  (return (`KismetArrayLibrary.Array_Length` (`self.Waypoints`))))

(fn `GetWaypointLocation`
  (params (Index :type Integer))
  (returns (Location :type "Vector Structure"))
  (return (`self.K2_GetActorLocation` (`|GetArrayItem` (`self.Waypoints`) Index))))

(fn `Spawn`
  (params (Enemy :type "Pawn Class Reference"))
  (bind _returnvalue (`|SpawnActorFromClass` Enemy (`self.GetTransform`) "AdjustIfPossibleButAlwaysSpawn" "MultiplyWithRoot" null null))
  (`/Game/JamContent/BPs/Components/BP_WavePathingComponent.Begin Pathing` (`self.GetComponentByClass` _returnvalue "/Game/JamContent/BPs/Components/BP_WavePathingComponent.BP_WavePathingComponent_C") self))

(fn `SpawnBatch`
  (params (Batch :type "/Game/JamContent/BPs/Structs/WaveBatch Structure"))
  (bind _returnvalue (`AddComponent|NODE_AddBP_WaveBatchSpawnerComponent-0`))
  (`/Game/JamContent/BPs/Components/BP_WaveBatchSpawnerComponent.Begin Spawning` _returnvalue self Batch))

(fn `SpawnWave`
  (params (Wave :type "/Game/JamContent/BPs/Structs/Wave Structure"))
  (bind _returnvalue (`AddComponent|NODE_AddBP_WaveSpawnerComponent-0`))
  (`/Game/JamContent/BPs/Components/BP_WaveSpawnerComponent.Begin Wave` _returnvalue self Wave))

(fn `UserConstructionScript`)

(fn `VisualizePath`
  (if (> (`self.GetWaypointCount`) 0)
    (`self.DrawPathSegment` (`self.K2_GetActorLocation`) (`self.GetWaypointLocation` 0))
    (for _index (range (+ (- (`self.GetWaypointCount`) 2) 1))
      (`self.DrawPathSegment` (`self.GetWaypointLocation` _index) (`self.GetWaypointLocation` (+ _index 1))))))