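; Grenade launcher projectile that bounces and explodes, dealing radial damage.
; On bounce, hitting a BP_PBaseEnemy detonates it immediately, while the first bounce off anything else lights a one-time fuse timer.
; ExplodeGrenade applies full damage across the radius with no falloff, spawns Niagara sparks, plays a sound at world origin rather than the grenade, then destroys the actor.
; Debug prints and a radius sphere trace the behavior.
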(event `self.ProjectileMovement.OnProjectileBounce`
  (params (ImpactResult :type "HitResult Structure (by ref)") (ImpactVelocity :type "Vector Structure (by ref)"))
  (if (`GameplayStatics.ObjectIsA` (`.HitActor` (`GameplayStatics.BreakHitResult` ImpactResult)) "/Game/JamContent/BPs/Pawns/BP_PBaseEnemy.BP_PBaseEnemy_C")
    (`KismetSystemLibrary.PrintString` "Direct Hit")
    (`self.ExplodeGrenade`)
    (elif (not (`self.FuseLit`))
      (set `self.FuseLit` true)
      (`KismetSystemLibrary.PrintString` "Fuse Lit")
      (`KismetSystemLibrary.K2_SetTimer` null "ExplodeGrenade" (`self.FuseTimer`)))))

(fn `ExplodeGrenade`
  (bind _returnvalue (`self.K2_GetActorLocation` self))
  (bind _returnvalue_2 (`GameplayStatics.ApplyRadialDamage` :`BaseDamage` (`self.Damage`) :`Origin` _returnvalue :`DamageRadius` (`self.ExplosionRadius`) :`DamageTypeClass` "/Script/Engine.DamageType" :`DamageCauser` self :`InstigatedByController` null :`bDoFullDamage` true))
  (`KismetSystemLibrary.PrintString` (`KismetStringLibrary.Conv_BoolToString` _returnvalue_2))
  (`NiagaraFunctionLibrary.SpawnSystemAtLocation` "/Game/JamContent/Art/FX/NS_ExplosionSparks.NS_ExplosionSparks" _returnvalue (struct) (1.0 1.0 1.0) true true "AutoRelease")
  (`KismetSystemLibrary.DrawDebugSphere` (`self.K2_GetActorLocation` self) (`self.ExplosionRadius`) 12 (struct :`R` 1.0 :`G` 1.0 :`B` 1.0 :`A` 1.0) 1.5)
  (`GameplayStatics.PlaySoundAtLocation` "/Game/JamContent/Art/Audio/SFX/Temp/grenadeExplosion.grenadeExplosion" (0.0 0.0 0.0) (struct) 1.0 1.0 0.0 null null null null)
  (`self.K2_DestroyActor`))

(fn `UserConstructionScript`)