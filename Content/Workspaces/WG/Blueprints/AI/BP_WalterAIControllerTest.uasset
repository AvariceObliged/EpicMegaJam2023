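; Test AI controller that walks its pawn along the waypoints of a BP_WalterPath actor, then destroys the pawn.
; BeginPlay finds the path actor in the level and copies its Waypoints array.
; On possess, it chains AIMoveTo calls through the waypoints in order, advancing only on success.
; A failed move has no handler, so the sequence stops there.
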(event `self.ReceiveBeginPlay`
  (bind _returnvalue (`GameplayStatics.GetActorOfClass` "/Game/Workspaces/WG/Blueprints/Actors/BP_WalterPath.BP_WalterPath_C"))
  (set `self.Waypoints` (`/Game/Workspaces/WG/Blueprints/Actors/BP_WalterPath.Waypoints` _returnvalue)))

(event `self.ReceivePossess`
  (params (PossessedPawn :type "Pawn Object Reference"))
  (if (< (`self.NextWaypoint`) (`KismetArrayLibrary.Array_Length` (`self.Waypoints`))) :!label _label
    (`|AIMoveTo` null (`self.K2_GetActorLocation` (`|GetArrayItem` (`self.Waypoints`) (`self.NextWaypoint`))) null
      (:`OnSuccess`
        (set `self.NextWaypoint` (+ (`self.NextWaypoint`) 1))
        (goto _label)))
    (else
      (`self.K2_DestroyActor` (`self.K2_GetPawn`)))))

(fn `NewFunction`)

(fn `UserConstructionScript`)